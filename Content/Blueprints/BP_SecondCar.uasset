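; Secondary car actor that appears with a random look and drives along Y while the player's BP_Car game is on.
; BeginPlay reveals one of three meshes, randomizes their materials and caches the player car.
; Tick steps Y by a fixed, frame-dependent amount through a swept move, with a timeline setting spawn height.
; Player overlap with either box destroys it after a delay; only SecondCarMesh overlap sets IsCarHit.
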(event OnComponentBeginOverlap(SecondCarMesh)
  (params (OverlappedComponent :type Primitive%20Component%20Object%20Reference) (OtherActor :type Actor%20Object%20Reference) (OtherComp :type Primitive%20Component%20Object%20Reference) (OtherBodyIndex :type Integer) (bFromSweep :type Boolean) (SweepResult :type Hit%20Result%20Structure%20%28by%20ref%29))
  ;[1 1 1] Setting event hit to true when the payer collides with a car
  (Utilities|Casting|CastToBP_Car OtherActor)
  (Variables|Default|SetisCarHit true))

(event OnComponentBeginOverlap(Box)
  (params (OverlappedComponent :type Primitive%20Component%20Object%20Reference) (OtherActor :type Actor%20Object%20Reference) (OtherComp :type Primitive%20Component%20Object%20Reference) (OtherBodyIndex :type Integer) (bFromSweep :type Boolean) (SweepResult :type Hit%20Result%20Structure%20%28by%20ref%29))
  ;[1 0.7261 0] Destroying the second car after x time
  (Utilities|Casting|CastToBP_Car OtherActor)
  (Utilities|FlowControl|Delay 1.0)
  (Actor|DestroyActor))

(event OnComponentBeginOverlap(Box1)
  (params (OverlappedComponent :type Primitive%20Component%20Object%20Reference) (OtherActor :type Actor%20Object%20Reference) (OtherComp :type Primitive%20Component%20Object%20Reference) (OtherBodyIndex :type Integer) (bFromSweep :type Boolean) (SweepResult :type Hit%20Result%20Structure%20%28by%20ref%29))
  ;[1 0.7261 0] Destroying the second car after x time
  (Utilities|Casting|CastToBP_Car OtherActor)
  (Utilities|FlowControl|Delay 1.0)
  (Actor|DestroyActor))

(event EventBeginPlay
  (bind _thirdcarmesh (Variables|Default|GetThirdCarMesh))
  (bind _fourthcarmodel (Variables|Default|GetFourthCarModel))
  (bind _secondcarmesh (Variables|Default|GetSecondCarMesh))
  (Utilities|FlowControl|Sequence
    (:then_0
      ;[1 1 1] Set random car mesh
      (bind _output_get (Variables|Default|SetSpawnedCar (Utilities|Array|MakeArray (Variables|Default|GetThirdCarMesh) (Variables|Default|GetSecondCarMesh) (Variables|Default|GetFourthCarModel))))
      (Rendering|SetVisibility (.OutItem (Utilities|Array|Random _output_get)) true false))
    (:then_1
      ;[1 0.1756 0.06586] Set random material for second car mesh
      (switch int (Math|Random|RandomInteger 5)
        (:0
          (Rendering|Material|SetMaterial _secondcarmesh 0 "/Game/Materials/m_secondarycar.m_secondarycar"))
        (:1
          (Rendering|Material|SetMaterial _secondcarmesh 0 "/Game/Materials/m_secondarycar2.m_secondarycar2"))
        (:2
          (Rendering|Material|SetMaterial _secondcarmesh 0 "/Game/Materials/m_secondarycar3.m_secondarycar3"))
        (:3
          (Rendering|Material|SetMaterial _secondcarmesh 0 "/Game/Materials/m_secondarycar4.m_secondarycar4"))
        (:4
          (Rendering|Material|SetMaterial _secondcarmesh 0 "/Game/Materials/m_secondarycar5.m_secondarycar5"))))
    (:then_2
      ;[1 1 1] Reference to the main car
      (bind _asbp_car (Utilities|Casting|CastToBP_Car (Game|Player|GetPlayerPawn 0)))
      (Variables|Default|SetAs%20BP%20Car _asbp_car))
    (:then_3
      ;[1 0.3275 0.509] Set random material for third car mesh
      (switch int (Math|Random|RandomInteger 6)
        (:0
          (Rendering|Material|SetMaterial _thirdcarmesh 0 "/Game/Materials/m_secondarycar.m_secondarycar"))
        (:1
          (Rendering|Material|SetMaterial _thirdcarmesh 0 "/Game/Materials/m_secondarycar2.m_secondarycar2"))
        (:2
          (Rendering|Material|SetMaterial _thirdcarmesh 0 "/Game/Materials/m_secondarycar3.m_secondarycar3"))
        (:3
          (Rendering|Material|SetMaterial _thirdcarmesh 0 "/Game/Materials/m_secondarycar4.m_secondarycar4"))
        (:4
          (Rendering|Material|SetMaterial _thirdcarmesh 0 "/Game/Materials/m_secondarycar5.m_secondarycar5"))
        (:5
          (Rendering|Material|SetMaterial _thirdcarmesh 0 "/Game/Textures/m_thirdcartexture.m_thirdcartexture"))))
    (:then_4
      ;[1 0.3275 0.509] Set random material for third car mesh
      (switch int (Math|Random|RandomInteger 6)
        (:0
          (Rendering|Material|SetMaterial _fourthcarmodel 0 "/Game/Materials/m_secondarycar.m_secondarycar"))
        (:1
          (Rendering|Material|SetMaterial _fourthcarmodel 0 "/Game/Materials/m_secondarycar2.m_secondarycar2"))
        (:2
          (Rendering|Material|SetMaterial _fourthcarmodel 0 "/Game/Materials/m_secondarycar3.m_secondarycar3"))
        (:3
          (Rendering|Material|SetMaterial _fourthcarmodel 0 "/Game/Materials/m_secondarycar4.m_secondarycar4"))
        (:4
          (Rendering|Material|SetMaterial _fourthcarmodel 0 "/Game/Materials/m_secondarycar5.m_secondarycar5"))
        (:5
          (Rendering|Material|SetMaterial _fourthcarmodel 0 "/Game/Textures/m_thirdcartexture.m_thirdcartexture"))))))

(event EventTick
  (params (DeltaSeconds :type Float%20%28single-precision%29))
  (bind _returnvalue (Transformation|GetActorLocation))
  (Utilities|FlowControl|Sequence
    (:then_0
      ;[1 1 1] SecondCarVelocity
      (if (Variables|/Game/Blueprints/BP_Car.BP_Car_C|GetisGameOn (Variables|Default|GetAs%20BP%20Car))
        (bind _result (Utilities|ManipulateFloatInternal (.y _returnvalue) (+ (.y _returnvalue) 2e+01))
          (:%20%20
            (bind _zspawnpos (Timeline|SpawningZanimation Play)
              (:Update
                (Transformation|SetActorLocation (Math|Vector|MakeVector (.x _returnvalue) _result (Math|Float|Lerp 0.0 1.0 _zspawnpos)) true false)))))))))

(fn ConstructionScript)