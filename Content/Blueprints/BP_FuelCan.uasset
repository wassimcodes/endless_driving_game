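; BP_FuelCan is a fuel can actor that shows or hides its mesh based on its position relative to the car.
; BeginPlay caches a reference to the BP_Car found in the level.
; Every Tick compares the signed Y-axis offset from car to can against a fixed threshold, hiding the mesh only while the can is farther ahead along positive Y.
; The file contains no pickup or refuel logic.
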(event EventTick
  (params (DeltaSeconds :type Float%20%28single-precision%29))
  (bind _fuelcanmesh (Variables|Default|GetFuelCanMesh))
  (Utilities|FlowControl|Sequence
    (:then_0
      ;[0.3248 0.5712 1] Setting distance constrictions for the fuel to be  visible depending on the distance between the car and the fuel can
      (if (<= (- (.Y (Math|Vector|BreakVector (Transformation|GetActorLocation))) (.Y (Math|Vector|BreakVector (Transformation|GetActorLocation (Variables|Default|GetCarRef))))) 7e+03)
        (Rendering|SetVisibility _fuelcanmesh true false)
        (else
          (Rendering|SetVisibility _fuelcanmesh false false))))))

(event EventBeginPlay
  ;[1 1 1] Accessing the car
  (bind _returnvalue (Actor|GetActorOfClass "/Game/Blueprints/BP_Car.BP_Car_C"))
  (Variables|Default|SetCarRef _returnvalue))

(fn ConstructionScript)