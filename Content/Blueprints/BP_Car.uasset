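; BP_Car is a car that drives itself along the world Y axis once the game is started.
; BeginPlay clears IsGameOn and the Startkey input sets it.
; While it is set, Tick feeds an incrementing counter into a clamped Lerp and adds the result to the Y location with a swept move.
; The step is capped and applied per frame, without delta-time scaling.
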(event EventBeginPlay
  (Variables|Default|SetisGameOn false))

(event EventTick
  (params (DeltaSeconds :type Float%20%28single-precision%29))
  (bind _returnvalue (Transformation|GetActorLocation))
  (Utilities|FlowControl|Sequence
    (:then_3
      ;[0.474 0.5781 1] Car Y Automatic Movement
      (if (Variables|Default|GetisGameOn)
        (bind _result (Math|Float|IncrementFloat (Variables|Default|Getstartingval))
          (:%20%20
            (bind _result_2 (Utilities|ManipulateFloatInternal (.y _returnvalue) (+ (.y _returnvalue) (Math|Float|Clamp(Float) (Math|Float|Lerp 0.0 3e+01 _result) 0.0 3e+01)))
              (:%20%20
                (Transformation|SetActorLocation (Math|Vector|MakeVector (.x _returnvalue) _result_2 (.z _returnvalue)) true false)))))))))

(event Input|ActionEvents|InputActionStartkey
  (params (Key :type Key%20Structure :default "None"))
  ;[1 0.5214 0.391] Starting The Game
  (:Pressed
    (Variables|Default|SetisGameOn true)))

(fn ConstructionScript)